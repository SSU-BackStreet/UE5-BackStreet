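; BP_ProjectileBase is a projectile actor, named as the base for weapon projectiles.
; Its construction script copies speed and gravity scale from ProjectileStat into ProjectileMovement, using one speed for both initial and max.
; Homing logic that would lock onto an overlapping "Character"-tagged actor other than the owner exists but is disconnected, so the TargetingCollision overlap event does nothing.
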(event OnComponentBeginOverlap(TargetingCollision)
  (params (OverlappedComponent :type Primitive%20Component%20Object%20Reference) (OtherActor :type Actor%20Object%20Reference) (OtherComp :type Primitive%20Component%20Object%20Reference) (OtherBodyIndex :type Integer) (bFromSweep :type Boolean) (SweepResult :type Hit%20Result%20Structure%20%28by%20ref%29)))

(fn ConstructionScript
  (bind _projectilemovement (Variables|Default|GetProjectileMovement))
  (bind _projectilestat (Variables|Default|GetProjectileStat))
  (bind (_projectilespeed _projectiledamage _gravityscale) (Utilities|Struct|BreakProjectileStatStruct _projectilestat))
  (Variables|/Script/Engine.ProjectileMovementComponent|SetInitialSpeed _projectilemovement _projectilespeed)
  (Variables|/Script/Engine.ProjectileMovementComponent|SetMaxSpeed _projectilemovement _projectilespeed)
  (Variables|/Script/Engine.ProjectileMovementComponent|SetProjectileGravityScale _projectilemovement _gravityscale))