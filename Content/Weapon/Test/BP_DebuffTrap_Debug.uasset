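; BP_DebuffTrap_Debug is a test trap actor that applies a configurable debuff to characters entering its box.
; The box's overlap event checks for a valid actor tagged "Character", casts it to CharacterBase and calls SetBuffTimer with the trap's debuff type, duration and variable, naming itself as causer.
; A DoOnce gate followed by a five-second delay and reset acts as a cooldown shared by all overlapping actors.
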(event OnComponentBeginOverlap(Box)
  (params (OverlappedComponent :type Primitive%20Component%20Object%20Reference) (OtherActor :type Actor%20Object%20Reference) (OtherComp :type Primitive%20Component%20Object%20Reference) (OtherBodyIndex :type Integer) (bFromSweep :type Boolean) (SweepResult :type Hit%20Result%20Structure%20%28by%20ref%29))
  (Utilities|IsValid OtherActor
    (:Is%20Valid
      (if (Actor|ActorHasTag OtherActor "Character")
        (Utilities|FlowControl|DoOnce false :!label _label
          (:Completed
            (Class|CharacterBase|SetBuffTimer (.AsCharacter%20Base (Utilities|Casting|CastToCharacterBase OtherActor)) true (Variables|Default|GetDebuff%20Type) self (Variables|Default|GetTotal%20Time) (Variables|Default|GetVariable))
            (Utilities|FlowControl|Delay 5.0)
            (goto _label Reset)))))))

(event EventBeginPlay)

(event Collision|EventActorBeginOverlap
  (params (OtherActor :type Actor%20Object%20Reference)))

(event EventTick
  (params (DeltaSeconds :type Float%20%28single-precision%29)))

(fn ConstructionScript)