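; Main character Blueprint whose only live logic is an on-screen debug readout of the character's current status.
; Tick calls PrintCharacterInfo, which loops over the debuff and buff enums to show active flags, then prints action state, attack ability, speed, defense, attack multiplier and HP.
; Short-duration colored prints, kept out of the log, refresh each frame like a live HUD.
; A mouse-cursor trace for facing direction is left unconnected.
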(event EventTick
  (params (DeltaSeconds :type Float%20%28single-precision%29))
  ;[0.9571 0 1 1 50] Tick / Debug
  (CallFunction|PrintCharacterInfo))

(event EventBeginPlay
  ;[0.9571 0 1 1 50] Tick / Debug
)

(fn ConstructionScript)

(fn PrintCharacterInfo
  (bind _characterstate (Variables|Default|GetCharacterState))
  (bind _characterstat (Variables|Default|GetCharacterStat))
  (bind (_characterdebuffstate _characterbuffstate _bcanattack _characteractionstate _charactercurrhp) (Utilities|Struct|BreakCharacterStateStruct _characterstate))
  (bind (_bisinvincibility _binfiniteammo _charactermaxhp _characteratkmultiplier _characteratkspeed _charactermovespeed _characterdefense) (Utilities|Struct|BreakCharacterStatStruct _characterstat))
  (Utilities|FlowControl|Sequence
    (:then_0
      (for _index (range 0 8)
        (LocalVariables|SetTemp (Utilities|String|Append (LocalVariables|GetTemp) (Utilities|String|Append (Utilities|String|EnumtoString (Utilities|Enum|ByteToEnumECharacterDebuffType (Math|Conversions|ToByte(Integer) _index))) " : " (Utilities|String|ToString(Boolean) (Class|CharacterBase|GetDebuffIsActive (Utilities|Enum|ByteToEnumECharacterDebuffType (Math|Conversions|ToByte(Integer) _index)))) " / "))))
      (Development|PrintString (LocalVariables|GetTemp) true false "(R=0.480775,G=1.000000,B=0.463542,A=1.000000)" 0.003)
      (LocalVariables|SetTemp ""))
    (:then_1
      (for _index_2 (range 0 8)
        (LocalVariables|SetTemp (Utilities|String|Append (LocalVariables|GetTemp) (Utilities|String|Append (Utilities|String|EnumtoString (Utilities|Enum|ByteToEnumECharacterBuffType (Math|Conversions|ToByte(Integer) _index_2))) " : " (Utilities|String|ToString(Boolean) (Class|CharacterBase|GetBuffIsActive (Utilities|Enum|ByteToEnumECharacterBuffType (Math|Conversions|ToByte(Integer) _index_2)))) " / "))))
      (Development|PrintString (LocalVariables|GetTemp) true false "(R=0.480775,G=1.000000,B=0.463542,A=1.000000)" 0.003)
      (LocalVariables|SetTemp ""))
    (:then_2
      (Development|PrintString (Utilities|String|Append "ActionState :  " (Utilities|String|EnumtoString _characteractionstate) "  /  Can Atk : " (Utilities|String|ToString(Boolean) _bcanattack)) true false "(R=1.000000,G=0.955652,B=0.000000,A=1.000000)" 0.003))
    (:then_3
      (Development|PrintString (Utilities|String|Append "Speed : " (Utilities|String|ToString(Float) (Variables|/Script/Engine.CharacterMovementComponent|GetMaxWalkSpeed (Variables|Character|GetCharacterMovement))) "/" (Utilities|String|ToString(Float) _charactermovespeed)) true false "(R=0.000000,G=0.900125,B=1.000000,A=1.000000)" 0.003))
    (:then_4
      (Development|PrintString (Utilities|String|Append "DEF : " (Utilities|String|ToString(Float) _characterdefense) "/ ATK : " (Utilities|String|ToString(Float) _characteratkmultiplier)) true false "(R=0.000000,G=0.363636,B=1.000000,A=1.000000)" 0.003))
    (:then_6
      (Development|PrintString (Utilities|String|Append "HP : " (Utilities|String|ToString(Float) _charactercurrhp) "/" (Utilities|String|ToString(Float) _charactermaxhp)) true false "(R=1.000000,G=0.227609,B=0.223958,A=1.000000)" 0.003))))